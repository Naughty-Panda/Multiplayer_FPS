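; BP_MultiplayerGameMode is a multiplayer game mode that names joining players and balances them across two teams.
; On PostLogin, it increments a player counter, gives the BP_MultiplayerPC a numbered "Player" name, and assigns it to the smaller team, favoring Team 1 on ties.
; On logout, it removes the controller from whichever team array holds it and prints a debug message.
; The player counter is never decremented, so name numbers keep climbing.
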(event EventBeginPlay)

(event EventTick
  (params (DeltaSeconds :type Float%20%28single-precision%29)))

(event EventOnLogout
  (params (ExitingController :type Controller%20Object%20Reference))
  (bind _asbp_multiplayer_pc (Utilities|Casting|CastToBP_MultiplayerPC ExitingController)
    (:then
      ;[1 1 1] Team 1 cleanup
      (bind _returnvalue (Utilities|Array|RemoveItem (Variables|Default|GetTeam1) _asbp_multiplayer_pc))
      (if _returnvalue
        (Development|PrintString "Team 1 Player disconnected..." true true "(R=1.000000,G=0.966854,B=0.867417,A=1.000000)" 1e+01)
        (else
          ;[1 1 1] Team 2 cleanup
          (bind _returnvalue_2 (Utilities|Array|RemoveItem (Variables|Default|GetTeam2) _asbp_multiplayer_pc))
          (if _returnvalue_2
            (Development|PrintString "Team 2 Player disconnected..." true true "(R=1.000000,G=0.966854,B=0.867417,A=1.000000)" 1e+01)
            (else
              (Development|PrintString "No player found in both teams..." true true "(R=1.000000,G=0.966854,B=0.867417,A=1.000000)" 1e+01))))))
    (:CastFailed
      (Development|PrintString "Logout: Bad cast!" true true "(R=1.000000,G=0.966854,B=0.867417,A=1.000000)" 1e+01))))

(event EventPostLogin
  (params (NewPlayer :type Player%20Controller%20Object%20Reference))
  (bind _asbp_multiplayer_pc (Utilities|Casting|CastToBP_MultiplayerPC NewPlayer)
    (:then
      (Math|Integer|IncrementInt (Variables|Default|GetCurrentPlayerCounter)
        (:%20%20
          (Default|SetPlayerName _asbp_multiplayer_pc (CallFunction|GeneratePlayerName))
          (if (> (Utilities|Array|Length (Variables|Default|GetTeam1)) (Utilities|Array|Length (Variables|Default|GetTeam2)))
            (Default|SetTeamID _asbp_multiplayer_pc 2)
            (Utilities|Array|Add (Variables|Default|GetTeam2) _asbp_multiplayer_pc)
            (else
              (Default|SetTeamID _asbp_multiplayer_pc 1)
              (Utilities|Array|Add (Variables|Default|GetTeam1) _asbp_multiplayer_pc))))))
    (:CastFailed
      (Development|PrintString "Error: wrong player controller!" true true "(R=1.000000,G=0.083333,B=0.083333,A=1.000000)" 1e+01))))

(fn ConstructionScript)

(fn GeneratePlayerName
  (return (Utilities|String|StringToName (Utilities|String|Append "Player " (Utilities|String|ToString(Integer) (Variables|Default|GetCurrentPlayerCounter))))))