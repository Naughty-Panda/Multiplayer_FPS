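; BP_Projectile is a networked projectile that flies straight along its forward vector and expires after a set lifetime.
; The server moves it each tick without sweeping and handles sphere overlaps, reacting only to characters or other projectiles and ignoring its owner.
; A valid hit multicasts an overlap-location event that spawns an emitter, then destroys the projectile through the same server event used by the lifetime timer.
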(event OnComponentBeginOverlap(Sphere)
  (params (OverlappedComponent :type Primitive%20Component%20Object%20Reference) (OtherActor :type Actor%20Object%20Reference) (OtherComp :type Primitive%20Component%20Object%20Reference) (OtherBodyIndex :type Integer) (bFromSweep :type Boolean) (SweepResult :type Hit%20Result%20Structure%20%28by%20ref%29))
  ;[1 1 1] Collision
  (if (Networking|IsServer)
    (CallFunction|ServerCollision OtherActor (Transformation|GetActorLocation))))

(event Custom|LifeEnded
  (CallFunction|ServerLifeEnded))

(event Custom|Server_LifeEnded
  (Actor|DestroyActor))

(event Custom|Server_Move
  (params (Delta%20Seconds :type Float%20%28double-precision%29))
  (Transformation|SetActorLocation (+ (Transformation|GetActorLocation) (* Delta%20Seconds (Transformation|GetActorForwardVector) (Variables|Default|GetSpeed))) false false))

(event Custom|Server_Collision
  (params (OtherActor :type Actor%20Object%20Reference) (Location :type Vector))
  ;[1 1 1] Collision
  (if (!= OtherActor (Components|GetOwner))
    (Utilities|Casting|CastToBP_BaseCharacter OtherActor
      (:then
        _)
      (:CastFailed
        (Utilities|Casting|CastToBP_Projectile OtherActor)))
    (CallFunction|MulticastHitEvent Location)
    (CallFunction|ServerLifeEnded)))

(event Custom|OnHitEvent
  (params (Location :type Vector))
  ;[1 1 1] Hit Event
  (Effects|SpawnEmitteratLocation 0 Location))

(event Custom|Multicast_HitEvent
  (params (Location :type Vector))
  ;[1 1 1] Hit Event
  (CallFunction|OnHitEvent Location))

(event EventBeginPlay
  (Utilities|Time|SetTimerbyEvent (delegate Custom|LifeEnded) (Variables|Default|GetTTL)))

(event EventTick
  (params (DeltaSeconds :type Float%20%28single-precision%29))
  (if (Networking|IsServer)
    (CallFunction|ServerMove DeltaSeconds)))

(fn ConstructionScript)