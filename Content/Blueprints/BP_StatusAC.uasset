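; BP_StatusAC is a status component that tracks its owner's health.
; CurrentHP starts at MaxHP on BeginPlay, and TakeDamage subtracts damage, clamped between zero and MaxHP.
; CurrentHP uses a RepNotify that casts the owner to BP_BaseCharacter, calls UpdateStatusBars and prints a debug string.
; GetPercentHP returns current health as a fraction of maximum.
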(event Custom|TakeDamage
  (params (Damage :type Float%20%28double-precision%29))
  (Variables|Default|SetCurrentHP (Math|Float|Clamp(Float) (- (Variables|Default|GetCurrentHP) Damage) 0.0 (Variables|Default|GetMaxHP))))

(event EventBeginPlay
  (Variables|Default|SetCurrentHP (Variables|Default|GetMaxHP)))

(event EventTick
  (params (DeltaSeconds :type Float%20%28single-precision%29)))

(fn OnRepCurrentHP
  (bind _asbp_base_character (Utilities|Casting|CastToBP_BaseCharacter (Components|GetOwner)))
  (Default|UpdateStatusBars _asbp_base_character)
  (Development|PrintString "OnRepHP")
  (return))

(fn GetPercentHP
  (return (/ (Variables|Default|GetCurrentHP) (Variables|Default|GetMaxHP))))