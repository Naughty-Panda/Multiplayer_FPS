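; Base multiplayer first-person character with projectile firing, damage and an overhead-style status widget showing name, team and health.
; On BeginPlay it tints its mesh by remote net role and sends the local controller's team and name to the server.
; The server setters wait a fixed delay for replication, then multicast a widget refresh.
; Firing spawns server projectiles, with a timed client callback re-enabling fire; damage goes to CharacterStatus.
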(event Custom|Server_Fire
  (params (SpawnTransform :type Transform))
  (bind _self self)
  ;[1 1 1] Fire and reloading
  (if true
    (Game|SpawnActorfromClass "/Game/Blueprints/BP_Projectile.BP_Projectile_C" SpawnTransform "AlwaysSpawn" _self _self)
    (Utilities|Time|SetTimerbyEvent (delegate Custom|ReloadTimer) (Variables|Default|GetReloadTime))))

(event Custom|TakeDamage
  (params (Damage :type Float%20%28double-precision%29))
  ;[1 1 1] Taking damage
  (Default|TakeDamage (Variables|Default|GetCharacterStatus) Damage)
  (Development|PrintString "Player taking damage..." true true "(R=1.000000,G=0.061974,B=0.052026,A=1.000000)"))

(event Custom|ReloadTimer
  ;[1 1 1] Fire and reloading
  (CallFunction|ClientReloading))

(event Custom|ClientReloading
  ;[1 1 1] Fire and reloading
  (Development|PrintString "Start reloading" true true "(R=0.348038,G=1.000000,B=0.118267,A=1.000000)")
  (Variables|Default|SetbCanFire true))

(event Custom|ServerSetTeamID
  (params (TeamID :type Byte))
  ;[1 1 1] Setting TeamID and PlayerName on the server
  (Variables|Default|SetTeamID TeamID)
  (Development|PrintString "ServSetID called!" true true "(R=0.000000,G=0.903073,B=1.000000,A=1.000000)" 3e+01)
  ;[1 1 1] Time to replicate TeamID to clients
  (Utilities|FlowControl|Delay 1.0)
  (CallFunction|MulticastChangedTeamID))

(event Custom|SetNameByTeam
  ;[1 1 1] After TeamID and PlayerName hes been replicated from the server, we can set it locally
  (Development|PrintString "SetID on Client" true true "(R=0.135731,G=1.000000,B=0.778513,A=1.000000)" 3e+01)
  (bind _aswbp_player_status (Utilities|Casting|CastToWBP_PlayerStatus (UserInterface|GetWidget (Variables|Default|GetStatusWidget))))
  (Default|SetPlayerName _aswbp_player_status (Utilities|Text|FormatText "{Name} Team {Team}" (Variables|Default|GetPlayerName) (Variables|Default|GetTeamID))))

(event Custom|MulticastChangedTeamID
  (Development|PrintString "MultiChangedID called!" true true "(R=0.000000,G=0.903073,B=1.000000,A=1.000000)" 3e+01)
  (CallFunction|SetNamebyTeam))

(event Custom|ServerSetPlayerName
  (params (PlayerName :type Name))
  ;[1 1 1] Setting TeamID and PlayerName on the server
  (Variables|Default|SetPlayerName PlayerName)
  ;[1 1 1] Time to replicate TeamID to clients
  (Utilities|FlowControl|Delay 1.0)
  (CallFunction|MulticastChangedTeamID))

(event EventBeginPlay
  (bind _returnvalue (Pawn|GetController))
  (bind _staticmesh (Variables|Default|GetStaticMesh))
  (bind _returnvalue_2 (Rendering|Material|CreateDynamicMaterialInstance _staticmesh 0 (Rendering|Material|GetMaterial _staticmesh 0) "None" :!class /Script/Engine.PrimitiveComponent))
  (Rendering|Material|SetVectorParameterValue _returnvalue_2 "SurfaceColor" (Utilities|Select :Index (Class|Actor|GetRemoteRole) :ROLE_None "(R=0.000000,G=0.000000,B=0.000000,A=1.000000)" :ROLE_SimulatedProxy "(R=0.885417,G=0.033468,B=0.000000,A=1.000000)" :ROLE_AutonomousProxy "(R=0.239097,G=0.703125,B=0.131038,A=1.000000)" :ROLE_Authority "(R=0.723958,G=0.067524,B=0.585318,A=1.000000)") :!class /Script/Engine.MaterialInstanceDynamic)
  (Utilities|FlowControl|Sequence
    (:then_0
      (Development|PrintString (Utilities|String|Append "PC: " (Utilities|GetDisplayName _returnvalue)) true true "(R=1.000000,G=0.866598,B=0.043423,A=1.000000)" 2e+01)
      (bind _asbp_multiplayer_pc (Utilities|Casting|CastToBP_MultiplayerPC _returnvalue)
        (:then
          ;[1 1 1] Controlled locally
          (Development|PrintString "Controlled locally" true true "(R=1.000000,G=0.858802,B=0.097049,A=1.000000)" 5e+01)
          (CallFunction|ServerSetTeamID (Variables|/Game/Blueprints/BP_MultiplayerPC.BP_MultiplayerPC_C|GetTeamID _asbp_multiplayer_pc))
          (CallFunction|ServerSetPlayerName (Variables|/Game/Blueprints/BP_MultiplayerPC.BP_MultiplayerPC_C|GetPlayerName _asbp_multiplayer_pc)))
        (:CastFailed
          ;[1 1 1] Controlled remotely
          (Development|PrintString "Controlled remotely" true true "(R=1.000000,G=0.561483,B=0.069179,A=1.000000)" 5e+01)
          (CallFunction|SetNamebyTeam))))
    (:then_1
      (CallFunction|UpdateStatusBars)
      (Variables|Default|SetbCanFire true))))

(event Collision|EventActorBeginOverlap
  (params (OtherActor :type Actor%20Object%20Reference)))

(event EventTick
  (params (DeltaSeconds :type Float%20%28single-precision%29)))

(event Input|MouseEvents|LeftMouseButton
  (params (Key :type Key%20Structure :default "None"))
  ;[1 1 1] Fire and reloading
  (:Pressed
    (if (Variables|Default|GetbCanFire)
      (CallFunction|ServerFire (Transformation|GetWorldTransform (Variables|Default|GetFirstPersonCameraComponent)))
      (Variables|Default|SetbCanFire false))))

(fn ConstructionScript)

(fn UpdateStatusBars
  (bind _aswbp_player_status (Utilities|Casting|CastToWBP_PlayerStatus (UserInterface|GetWidget (Variables|Default|GetStatusWidget))))
  (Default|UpdateBars _aswbp_player_status (Default|GetPercentHP (Variables|Default|GetCharacterStatus))))