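; Game instance that hosts, finds and joins LAN multiplayer sessions.
; CreateGame creates a session, then opens OpenWorld as a listen server.
; FindSessions stores results, printing details and calling OnSessionFound for each, while JoinSession validates the given index but always joins the first result.
; Session failures, network errors and travel errors are reported with on-screen prints.
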(event Custom|CreateGame
  ;[1 1 1] Create Session and open level
  (|Session (Game|GetPlayerController 0) 16 true
    (:OnSuccess
      (Game|OpenLevel(byName) "OpenWorld" true "listen"))
    (:OnFailure
      (Development|PrintString "Error creating session!" true true "(R=1.000000,G=0.000000,B=0.009645,A=1.000000)" 1e+01))))

(event Custom|FindSessions
  ;[1 1 1] Find session
  (bind _results (|FindSessions (Game|GetPlayerController 0) 10 true)
    (:OnSuccess
      (bind _output_get (Variables|Default|SetFoundSessions _results))
      (for _array_element _output_get
        (Development|PrintString (Utilities|String|Append "Server: " (Class|FindSessionsCallbackProxy|GetServerName _array_element) " Ping: " (Utilities|String|ToString(Integer) (Class|FindSessionsCallbackProxy|GetPinginMs _array_element)) " Players: " (Utilities|String|ToString(Integer) (Class|FindSessionsCallbackProxy|GetCurrentPlayers _array_element)) "/" (Utilities|String|ToString(Integer) (Class|FindSessionsCallbackProxy|GetMaxPlayers _array_element))) true true "(R=0.174184,G=1.000000,B=0.133474,A=1.000000)" 1e+01)
        (Default|CallOnSessionFound)))
    (:OnFailure
      (Development|PrintString "Error finding session!" true true "(R=1.000000,G=0.106016,B=0.016356,A=1.000000)" 1e+01))))

(event Custom|JoinSession
  (params (SessionIndex :type Integer))
  (bind _foundsessions (Variables|Default|GetFoundSessions))
  ;[1 1 1] Join session
  (if (Utilities|Array|IsValidIndex _foundsessions SessionIndex)
    (|JoinSession (Game|GetPlayerController 0) (Utilities|Array|Get(acopy) _foundsessions)
      (:OnFailure
        (Development|PrintString "Error joining session!" true true "(R=1.000000,G=0.029832,B=0.000000,A=1.000000)" 1e+01)))
    (else
      (Development|PrintString "Error: invalid session idx!"))))

(event EventHandleNetworkError
  (params (FailureType :type ENetworkFailure%20Enum :default "NetDriverAlreadyExists") (bIsServer :type Boolean))
  ;[1 0.2864 0.2266] Network error handling
  (Development|PrintText (Utilities|Text|FormatText "Network Error: {NetErr} {IsServer}" (Utilities|Text|ToText(String) FailureType) (Utilities|Text|ToText(String) (Utilities|String|SelectString "on server!" "on client!" bIsServer)))))

(event EventHandleTravelError
  (params (FailureType :type ETravelFailure%20Enum :default "NoLevel"))
  ;[1 0.2864 0.2266] Network error handling
  (Development|PrintText (Utilities|Text|FormatText "Network travel error: {NetTravelErr}" (Utilities|Text|ToText(String) FailureType))))